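; BP_Car is a drivable physics car built on forces applied to a Collider, using Enhanced Input.
; Each Tick, a downward trace per wheel applies spring-like suspension force and offsets the wheel's child component.
; Every wheel pushes the body forward by smoothed throttle, even airborne; only new throttle input is ground-checked.
; Steering adds throttle-scaled yaw torque and turns the front wheels, while decaying throttle also drives wheel spin.
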(event Input|EnhancedActionEvents|EnhancedInputActionIA_Accelerate
  (params (ActionValue :type Float%20%28double-precision%29) (ElapsedSeconds :type Float%20%28double-precision%29) (TriggeredSeconds :type Float%20%28double-precision%29) (InputAction :type Input%20Action%20Object%20Reference :default "/Game/Vehicle_Movement/Inputs/IA_Accelerate.IA_Accelerate"))
  (Variables|Default|SetAccelerationInput (Math|Interpolation|FInterpTo (Variables|Default|GetAccelerationInput) (Math|Float|SelectFloat ActionValue 0.0 (CallFunction|IsonGround)) (Utilities|Time|GetWorldDeltaSeconds) 0.5)))

(event Input|EnhancedActionEvents|EnhancedInputActionIA_Steer
  (params (ActionValue :type Float%20%28double-precision%29) (ElapsedSeconds :type Float%20%28double-precision%29) (TriggeredSeconds :type Float%20%28double-precision%29) (InputAction :type Input%20Action%20Object%20Reference :default "/Game/Vehicle_Movement/Inputs/IA_Steer.IA_Steer"))
  (Class|PrimitiveComponent|AddTorqueinRadians (Variables|Default|GetCollider) (Math|Vector|MakeVector 0.0 0.0 (* ActionValue 5e+07 (Variables|Default|GetAccelerationInput))) "None" false)
  (Transformation|SetRelativeRotation (Variables|Default|GetFL_Wheel) (Math|Rotator|MakeRotator 0.0 0.0 (Math|Interpolation|FInterpTo (.yaw (Variables|/Script/Engine.SceneComponent|GetRelativeRotation (Variables|Default|GetFR_Wheel))) ActionValue (Utilities|Time|GetWorldDeltaSeconds) 3.0)) false false))

(event EventTick
  (params (DeltaSeconds :type Float%20%28single-precision%29))
  (CallFunction|SuspentionCast (Variables|Default|GetFL_Wheel))
  (CallFunction|SuspentionCast (Variables|Default|GetFR_Wheel))
  (CallFunction|SuspentionCast (Variables|Default|GetBL_Wheel))
  (CallFunction|SuspentionCast (Variables|Default|GetBR_Wheel))
  (CallFunction|CalculateAcceleration))

(event EventBeginPlay
  (Input|AddMappingContext (PlayerController|LocalPlayerSubsystems|GetEnhancedInputLocalPlayerSubsystem (Game|GetPlayerController 0)) "/Game/Vehicle_Movement/Inputs/IMC_Vehicle.IMC_Vehicle" 0 "(bIgnoreAllPressedKeysUntilRelease=True,bForceImmediately=False,bNotifyUserSettings=False)"))

(fn ConstructionScript)

(fn SuspentionCast
  (params (WheelComp :type Scene%20Component%20Object%20Reference))
  (bind _returnvalue (Transformation|GetWorldLocation WheelComp))
  (bind _returnvalue_2 (Components|GetChildComponent WheelComp 0))
  (bind _outhit (Collision|LineTraceByChannel _returnvalue (+ _returnvalue (* (Math|Vector|GetUpVector WheelComp) -6e+01)) "TraceTypeQuery1" false 0 "ForOneFrame"))
  (if (.bBlockingHit (Collision|BreakHitResult _outhit))
    (Class|PrimitiveComponent|AddForceatLocation (Variables|Default|GetCollider) (* (- 1.0 (Math|Float|NormalizetoRange (.Distance (Collision|BreakHitResult _outhit)) 0.0 6e+01)) (Math|Vector|GetUnitDirection(Vector) (.TraceEnd (Collision|BreakHitResult _outhit)) (.TraceStart (Collision|BreakHitResult _outhit))) 1e+06) (Transformation|GetWorldLocation WheelComp) "None")
    (CallFunction|AccelerateCar WheelComp)
    (Transformation|SetRelativeLocation _returnvalue_2 (Math|Vector|MakeVector 0.0 0.0 (Math|Interpolation|FInterpTo (.z (Variables|/Script/Engine.SceneComponent|GetRelativeLocation _returnvalue_2)) (+ (* (.Distance (Collision|BreakHitResult _outhit)) -1.0) 47.0) (Utilities|Time|GetWorldDeltaSeconds) 3.0)) false false)
    (else
      (CallFunction|AccelerateCar WheelComp))))

(fn CalculateAcceleration
  (bind _output_get (Variables|Default|SetAcceleration (* (Math|Float|Lerp 0.0 1.5e+04 (Variables|Default|GetAccelerationInput)) (Variables|Default|GetAccelerationInput))))
  (Variables|Default|SetAccelerationInput (Math|Interpolation|FInterpTo (Variables|Default|GetAccelerationInput) 0.0 (Utilities|Time|GetWorldDeltaSeconds) 0.3))
  (Transformation|AddLocalRotation (Variables|Default|GetWheel_FR) (Math|Rotator|MakeRotator 0.0 (/ _output_get -1e+03) 0.0) false false))

(fn AccelerateCar
  (params (WheelComp :type Scene%20Component%20Object%20Reference))
  (bind _collider (Variables|Default|GetCollider))
  (Class|PrimitiveComponent|AddForceatLocation (Variables|Default|GetCollider) (* (Math|Vector|GetForwardVector _collider) 1e+03 (Variables|Default|GetAccelerationInput) (Physics|GetMass _collider)) (Transformation|GetWorldLocation WheelComp) "None"))

(fn IsonGround
  (bind _returnvalue (Transformation|GetActorLocation))
  (bind _returnvalue_2 (Collision|LineTraceByChannel _returnvalue (- _returnvalue "0.000000,0.000000,100.000000") "TraceTypeQuery1" false 0 "None"))
  (return _returnvalue_2))