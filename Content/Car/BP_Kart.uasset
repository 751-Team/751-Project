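; Player kart pawn for a race game with a build phase, driven by forces on a physics box.
; Each tick, four wheel traces apply spring suspension, drive force is added even airborne, airborne wheels add selectable extra gravity, and pitch and roll ease level.
; Enhanced Input feeds steering torque and smoothed throttle.
; It also hands possession to a top-down builder, resets to its start, and cycles spectator views after finishing.
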(event Custom|RedoControlls
  (Transformation|SetActorTransform (Variables|Default|GetStart%20Locatoin))
  (bind _asplayer_controller (Utilities|Casting|CastToPlayerController (Pawn|GetController)))
  (Input|RemoveMappingContext (PlayerController|LocalPlayerSubsystems|GetEnhancedInputLocalPlayerSubsystem _asplayer_controller) "/Game/Trap_System/TopDownView/Inputs/IM_Movement.IM_Movement" "(bIgnoreAllPressedKeysUntilRelease=True,bForceImmediately=False,bNotifyUserSettings=False)")
  (Input|AddMappingContext (PlayerController|LocalPlayerSubsystems|GetEnhancedInputLocalPlayerSubsystem _asplayer_controller) "/Game/Car/Inputs/IMC_Kart.IMC_Kart" 0 "(bIgnoreAllPressedKeysUntilRelease=True,bForceImmediately=False,bNotifyUserSettings=False)")
  (Collision|SetCollisionEnabled (Variables|Default|GetBox) "QueryAndPhysics")
  (Variables|Default|SetIsBuilding false)
  (Variables|Default|SetFinishedRace false)
  (Class|PrimitiveComponent|SetAllPhysicsLinearVelocity (Variables|Default|GetBox) "0, 0, 0" false))

(event Custom|BuildingPhase
  (Variables|Default|SetIsBuilding true)
  (Class|PrimitiveComponent|SetAllPhysicsLinearVelocity (Variables|Default|GetWheel_BR) "0, 0, 0" false)
  (Collision|SetCollisionEnabled (Variables|Default|GetBox) "QueryAndPhysics")
  (bind _returnvalue (Game|SpawnActorfromClass "/Game/Trap_System/TopDownView/BP_Topdown.BP_Topdown_C" (stale EventBeginPlay _output_get) "Undefined" "MultiplyWithRoot" 0 0))
  (bind _asplayer_controller (Utilities|Casting|CastToPlayerController (Pawn|GetController)))
  (Pawn|Possess _asplayer_controller _returnvalue)
  (Default|SetKartMaster (Variables|/Game/Trap_System/TopDownView/BP_Topdown.BP_Topdown_C|GetBPC_BuildSystem _returnvalue) self)
  (Default|BeginBuild (Variables|/Game/Trap_System/TopDownView/BP_Topdown.BP_Topdown_C|GetBPC_BuildSystem _returnvalue)))

(event Custom|NextPlayerSpec
  (bind _asstate_race (Utilities|Casting|CastToState_Race (Game|GetGameState)))
  (bind _asplayer_controller (Utilities|Casting|CastToPlayerController (Pawn|GetController)))
  (if (== (+ (Variables|Default|GetCurrentPlayerSpectate) 1) (Utilities|Array|Length (Variables|/Game/Gamemode/State_Race.State_Race_C|GetPlayers _asstate_race)))
    (Variables|Default|SetCurrentPlayerSpectate 0)
    (else
      (Variables|Default|SetCurrentPlayerSpectate (+ (Variables|Default|GetCurrentPlayerSpectate) 1))))
  (if (== (Variables|Default|GetCurrentPlayerSpectate) (Variables|Default|GetPlayerID))
    (if (== (+ (Variables|Default|GetCurrentPlayerSpectate) 1) (Utilities|Array|Length (Variables|/Game/Gamemode/State_Race.State_Race_C|GetPlayers _asstate_race)))
      (Variables|Default|SetCurrentPlayerSpectate 0)
      (else
        (Variables|Default|SetCurrentPlayerSpectate (+ (Variables|Default|GetCurrentPlayerSpectate) 1)))))
  (Game|Player|SetViewTargetwithBlend _asplayer_controller (Utilities|Array|Get(acopy) (Variables|/Game/Gamemode/State_Race.State_Race_C|GetPlayers _asstate_race) (Variables|Default|GetCurrentPlayerSpectate)) 0.0 "VTBlend_Linear" 0.0 false))

(event Input|EnhancedActionEvents|EnhancedInputActionIA_Accelrate
  (params (ActionValue :type Float%20%28double-precision%29) (ElapsedSeconds :type Float%20%28double-precision%29) (TriggeredSeconds :type Float%20%28double-precision%29) (InputAction :type Input%20Action%20Object%20Reference :default "/Game/Car/Inputs/IA_Accelrate.IA_Accelrate"))
  (if (not (Variables|Default|GetFinishedRace))
    (Variables|Default|SetAccelerationInput (Math|Interpolation|FInterpTo (Variables|Default|GetAccelerationInput) ActionValue (Utilities|Time|GetWorldDeltaSeconds) 0.5))))

(event Input|EnhancedActionEvents|EnhancedInputActionIA_Steer
  (params (ActionValue :type Float%20%28double-precision%29) (ElapsedSeconds :type Float%20%28double-precision%29) (TriggeredSeconds :type Float%20%28double-precision%29) (InputAction :type Input%20Action%20Object%20Reference :default "/Game/Car/Inputs/IA_Steer.IA_Steer"))
  (if (not (Variables|Default|GetFinishedRace))
    (Class|PrimitiveComponent|AddTorqueinRadians (Variables|Default|GetBox) (* (Math|Vector|GetUpVector (Variables|Default|GetBox)) (* ActionValue (Variables|Default|GetTorqueTurn))) "None" false)
    (Transformation|SetRelativeRotation (Variables|Default|GetFL_wheel) (Math|Rotator|MakeRotator 0.0 0.0 (Math|Interpolation|FInterpTo (.yaw (Variables|/Script/Engine.SceneComponent|GetRelativeRotation (Variables|Default|GetFR_wheel))) ActionValue (Utilities|Time|GetWorldDeltaSeconds) 3.0)) false false)))

(event Input|EnhancedActionEvents|EnhancedInputActionSpecateNext
  (params (ActionValue :type Boolean) (ElapsedSeconds :type Float%20%28double-precision%29) (TriggeredSeconds :type Float%20%28double-precision%29) (InputAction :type Input%20Action%20Object%20Reference :default "/Game/Car/Inputs/SpecateNext.SpecateNext"))
  (if (Variables|Default|GetFinishedRace)
    (bind _asstate_race (Utilities|Casting|CastToState_Race (Game|GetGameState)))
    (bind _asplayer_controller (Utilities|Casting|CastToPlayerController (Pawn|GetController)))
    (if (== (+ (Variables|Default|GetCurrentPlayerSpectate) 1) (Utilities|Array|Length (Variables|/Game/Gamemode/State_Race.State_Race_C|GetPlayers _asstate_race)))
      (Variables|Default|SetCurrentPlayerSpectate 0)
      (else
        (Variables|Default|SetCurrentPlayerSpectate (+ (Variables|Default|GetCurrentPlayerSpectate) 1))))
    (if (== (Variables|Default|GetCurrentPlayerSpectate) (Variables|Default|GetPlayerID))
      (if (== (+ (Variables|Default|GetCurrentPlayerSpectate) 1) (Utilities|Array|Length (Variables|/Game/Gamemode/State_Race.State_Race_C|GetPlayers _asstate_race)))
        (Variables|Default|SetCurrentPlayerSpectate 0)
        (else
          (Variables|Default|SetCurrentPlayerSpectate (+ (Variables|Default|GetCurrentPlayerSpectate) 1)))))
    (Game|Player|SetViewTargetwithBlend _asplayer_controller (Utilities|Array|Get(acopy) (Variables|/Game/Gamemode/State_Race.State_Race_C|GetPlayers _asstate_race) (Variables|Default|GetCurrentPlayerSpectate)) 0.0 "VTBlend_Linear" 0.0 false)))

(event Input|EnhancedActionEvents|EnhancedInputActionSpectatePre
  (params (ActionValue :type Boolean) (ElapsedSeconds :type Float%20%28double-precision%29) (TriggeredSeconds :type Float%20%28double-precision%29) (InputAction :type Input%20Action%20Object%20Reference :default "/Game/Car/Inputs/SpectatePre.SpectatePre"))
  (if (Variables|Default|GetFinishedRace)
    (bind _asstate_race (Utilities|Casting|CastToState_Race (Game|GetGameState)))
    (bind _asplayer_controller (Utilities|Casting|CastToPlayerController (Pawn|GetController)))
    (if (== (- (Variables|Default|GetCurrentPlayerSpectate) 1) -1)
      (Variables|Default|SetCurrentPlayerSpectate (- (Utilities|Array|Length (Variables|/Game/Gamemode/State_Race.State_Race_C|GetPlayers _asstate_race)) 1))
      (else
        (Variables|Default|SetCurrentPlayerSpectate (- (Variables|Default|GetCurrentPlayerSpectate) 1))))
    (if (== (Variables|Default|GetCurrentPlayerSpectate) (Variables|Default|GetPlayerID))
      (if (== (- (Variables|Default|GetCurrentPlayerSpectate) 1) -1)
        (Variables|Default|SetCurrentPlayerSpectate (- (Utilities|Array|Length (Variables|/Game/Gamemode/State_Race.State_Race_C|GetPlayers _asstate_race)) 1))
        (else
          (Variables|Default|SetCurrentPlayerSpectate (- (Variables|Default|GetCurrentPlayerSpectate) 1)))))
    (Game|Player|SetViewTargetwithBlend _asplayer_controller (Utilities|Array|Get(acopy) (Variables|/Game/Gamemode/State_Race.State_Race_C|GetPlayers _asstate_race) (Variables|Default|GetCurrentPlayerSpectate)) 0.0 "VTBlend_Linear" 0.0 false)))

(event EventBeginPlay
  (Utilities|FlowControl|Sequence
    (:then_0
      (Utilities|FlowControl|Delay 0.2)
      (bind _asplayer_controller (Utilities|Casting|CastToPlayerController (Pawn|GetController)))
      (Input|AddMappingContext (PlayerController|LocalPlayerSubsystems|GetEnhancedInputLocalPlayerSubsystem _asplayer_controller) "/Game/Car/Inputs/IMC_Kart.IMC_Kart" 0 "(bIgnoreAllPressedKeysUntilRelease=True,bForceImmediately=False,bNotifyUserSettings=False)")
      (bind _output_get (Variables|Default|SetStart%20Locatoin (Transformation|GetActorTransform)))
      (bind _asstate_race (Utilities|Casting|CastToState_Race (Game|GetGameState)))
      (bind _returnvalue (UserInterface|CreateWidget "/Game/Gamemode/Timer.Timer_C" _asplayer_controller))
      (UserInterface|Viewport|AddtoPlayerScreen _returnvalue))))

(event Collision|EventActorBeginOverlap
  (params (OtherActor :type Actor%20Object%20Reference)))

(event EventTick
  (params (DeltaSeconds :type Float%20%28single-precision%29))
  (Utilities|FlowControl|Sequence
    (:then_0
      (CallFunction|SuspensionCast (Variables|Default|GetFR_wheel))
      (CallFunction|SuspensionCast (Variables|Default|GetFL_wheel))
      (CallFunction|SuspensionCast (Variables|Default|GetBR_wheel))
      (CallFunction|SuspensionCast (Variables|Default|GetBL_wheel))
      (CallFunction|CalculateAcceleration)
      (CallFunction|KeepRotatedCorrectly))
    (:then_1
      (CallFunction|GravityFalls (Variables|Default|GetFR_wheel))
      (CallFunction|GravityFalls (Variables|Default|GetFL_wheel))
      (CallFunction|GravityFalls (Variables|Default|GetBR_wheel))
      (CallFunction|GravityFalls (Variables|Default|GetBL_wheel)))))

(fn ConstructionScript)

(fn SuspensionCast
  (params (Wheel%20Comp :type Scene%20Component%20Object%20Reference))
  (bind _returnvalue (Transformation|GetWorldLocation Wheel%20Comp))
  (bind _outhit (Collision|LineTraceByChannel _returnvalue (+ _returnvalue (* (Math|Vector|GetUpVector Wheel%20Comp) -1e+02)) "TraceTypeQuery1" false 0 "None"))
  (if (.bBlockingHit (Collision|BreakHitResult _outhit))
    (Class|PrimitiveComponent|AddForceatLocation (Variables|Default|GetBox) (* (- 1.0 (Math|Float|NormalizetoRange (.Distance (Collision|BreakHitResult _outhit)) 0.0 3e+01)) (Math|Vector|GetUnitDirection(Vector) (.TraceEnd (Collision|BreakHitResult _outhit)) (.TraceStart (Collision|BreakHitResult _outhit))) 9e+04) (Transformation|GetWorldLocation Wheel%20Comp) "None")
    (CallFunction|AccelerateKart Wheel%20Comp)
    (else
      (CallFunction|AccelerateKart Wheel%20Comp))))

(fn CalculateAcceleration
  (bind _output_get (Variables|Default|SetAcceleration (Math|Float|Lerp 0.0 1.5e+04 (Variables|Default|GetAccelerationInput))))
  (Variables|Default|SetAccelerationInput (Math|Interpolation|FInterpTo (Variables|Default|GetAccelerationInput) 0.0 (Utilities|Time|GetWorldDeltaSeconds) 0.3))
  (Transformation|AddLocalRotation (Variables|Default|GetWheel_BR) (Math|Rotator|MakeRotator 0.0 (/ _output_get -1e+03) 0.0) false false))

(fn AccelerateKart
  (params (Wheel%20Comp :type Scene%20Component%20Object%20Reference))
  (bind _box (Variables|Default|GetBox))
  (Class|PrimitiveComponent|AddForceatLocation _box (* (* (Math|Vector|GetForwardVector _box) (* 1.0 1e+03) (Variables|Default|GetAccelerationInput) (Physics|GetMass _box)) (Variables|Default|GetmultiSpeed)) (Transformation|GetWorldLocation Wheel%20Comp) "None"))

(fn IsonGround
  (bind _groundcheck (Variables|Default|GetGroundCheck))
  (bind _returnvalue (Transformation|GetWorldLocation _groundcheck))
  (bind _returnvalue_2 (Collision|LineTraceByChannel _returnvalue (- _returnvalue "0.000000,0.000000,60.000000") "TraceTypeQuery1" false 0 "None"))
  (return _returnvalue_2))

(fn KeepRotatedCorrectly
  (bind _returnvalue (Utilities|Time|GetWorldDeltaSeconds))
  (bind _box (Variables|Default|GetBox))
  (bind _returnvalue_2 (Transformation|GetWorldRotation _box))
  (Transformation|SetWorldRotation _box (Math|Rotator|MakeRotator (Math|Interpolation|FInterpTo (.roll _returnvalue_2) 0.0 _returnvalue 1.0) (Math|Interpolation|FInterpTo (.pitch _returnvalue_2) 0.0 _returnvalue 1.0) (.yaw _returnvalue_2)) false false))

(fn IsonGroundWheels
  (params (Target :type Scene%20Component%20Object%20Reference))
  (bind _returnvalue (Transformation|GetWorldLocation Target))
  (bind _returnvalue_2 (Collision|LineTraceByChannel _returnvalue (+ (* (Math|Vector|GetUpVector Target) -1e+02) _returnvalue) "TraceTypeQuery1" false 0 "None"))
  (return _returnvalue_2))

(fn GravityFalls
  (params (Target :type Scene%20Component%20Object%20Reference))
  (bind _returnvalue (Transformation|GetWorldLocation Target))
  (bind _box (Variables|Default|GetBox))
  (bind _gravity_multiplier (Variables|Default|GetGravity%20Multiplier))
  (bind _returnvalue_2 (* _gravity_multiplier -1e+05))
  (bind _returnvalue_3 (* _gravity_multiplier -2.5e+03))
  (if (not (CallFunction|IsonGroundWheels Target))
    (switch int (- (Variables|Default|GetGravityOption) 1)
      (:Default
        (Class|PrimitiveComponent|AddForceatLocation _box (Math|Vector|MakeVector 0.0 0.0 _returnvalue_2) _returnvalue "None" :!label _label))
      (:0
        (goto _label))
      (:1
        (Physics|AddForce _box (Math|Vector|MakeVector 0.0 0.0 _returnvalue_2) "None" false))
      (:2
        (Physics|AddImpulse _box (Math|Vector|MakeVector 0.0 0.0 _returnvalue_3) "None" false))
      (:3
        (Physics|AddImpulseatLocation _box (Math|Vector|MakeVector 0.0 0.0 _returnvalue_3) _returnvalue "None")))))