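; BP_Cactus_03 is a Wild West cactus prop that plays an impact sound when a BP_Kart hits it.
; The Hit event plays the sound at the hit location, with clamped volume derived from the X component of the kart Box's velocity.
; A DoOnce that resets after a short delay keeps repeated hits from stacking sounds.
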(event EventBeginPlay)

(event Collision|EventActorBeginOverlap
  (params (OtherActor :type Actor%20Object%20Reference)))

(event EventTick
  (params (DeltaSeconds :type Float%20%28single-precision%29)))

(event Collision|EventHit
  (params (MyComp :type Primitive%20Component%20Object%20Reference) (Other :type Actor%20Object%20Reference) (OtherComp :type Primitive%20Component%20Object%20Reference) (bSelfMoved :type Boolean) (HitLocation :type Vector :default "0, 0, 0") (HitNormal :type Vector :default "0, 0, 0") (NormalImpulse :type Vector :default "0, 0, 0") (Hit :type Hit%20Result%20Structure%20%28by%20ref%29))
  (bind _asbp_kart (Utilities|Casting|CastToBP_Kart Other))
  (Utilities|FlowControl|DoOnce false :!label _label
    (:Completed
      (Audio|PlaySoundatLocation "/Game/Audio/Traps/Cactus_Hit.Cactus_Hit" HitLocation "0, 0, 0" (Math|Float|Clamp(Float) (/ (Math|Vector|VectorLength (Math|Conversions|ToVector(Float) (.X (Math|Vector|BreakVector (Transformation|GetComponentVelocity (Variables|/Game/Car/BP_Kart.BP_Kart_C|GetBox _asbp_kart)))))) 1e+01) 0.0 0.85) 1.0 0.0 0 0 0 0)
      (Utilities|FlowControl|Delay 0.4)
      (goto _label Reset))))

(fn ConstructionScript)