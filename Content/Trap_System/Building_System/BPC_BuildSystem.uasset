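; Component on BP_Topdown that runs trap selection and grid-based placement on the track in a kart racing game.
; BeginBuild opens the selection widget and creates a preview mesh, and State_Race tracks picked traps and finished players.
; A camera trace snaps the rotatable preview to the grid, while a box trace blocks placement on traps or off-track.
; Placing spawns the trap through RPC events, and ChangeToKart returns control to the kart.
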(event Custom|Preview%20Loop
  (bind _build_preview_rotation (Variables|Default|GetBuild%20Preview%20Rotation))
  (bind _preview_mesh (Variables|Default|GetPreview%20Mesh))
  (bind _boxtracehalfsize (Variables|Default|GetBoxTraceHalfSize))
  (bind _camera (Variables|Default|GetCamera))
  (bind _returnvalue (Transformation|GetWorldTransform _camera))
  ;[0.15 0.15 0.15 0.5] Look from camera centre OLD
  (bind _outactors (Actor|GetAllActorsOfClass "/Game/Trap_System/Traps/BP_TrapMaster.BP_TrapMaster_C"))
  (bind (_outhit _returnvalue_2) (Collision|LineTraceByChannel (.location _returnvalue) (+ (.location _returnvalue) (* (Math|Vector|GetForwardVector (.rotation _returnvalue)) 2e+03)) "TraceTypeQuery1" false _outactors "None"))
  (bind _location_on_grid (CallFunction|GetGridLocation (.Location (Collision|BreakHitResult _outhit))))
  (Utilities|FlowControl|Sequence
    (:then_1
      (bind _output_get (Variables|Default|SetBuild%20Preview%20Transform (Math|Transform|MakeTransform _location_on_grid _build_preview_rotation "1.000000,1.000000,1.000000")))
      (bind _outactors_2 (Actor|GetAllActorsOfClass "/Game/Trap_System/TopDownView/BP_Topdown.BP_Topdown_C"))
      (bind _outhit_2 (Collision|BoxTraceByChannel (+ _location_on_grid "0.000000,0.000000,100.000000") _location_on_grid (Math|Vector|MakeVector (- (.x _boxtracehalfsize) 1.0) (- (.y _boxtracehalfsize) 1.0) 0.0) _build_preview_rotation "TraceTypeQuery3" false _outactors_2 "None" true "(R=1.000000,G=0.000000,B=0.969969,A=1.000000)" "(R=1.000000,G=0.894132,B=0.000000,A=1.000000)"))
      (Utilities|FlowControl|Sequence
        (:then_1
          (if (or (Utilities|ClassIsChildOf (Utilities|GetClass (.hitactor _outhit_2)) "/Game/Trap_System/Traps/BP_TrapMaster.BP_TrapMaster_C") (not (Utilities|ClassIsChildOf (Utilities|GetClass (.hitactor _outhit_2)) "/Game/Trap_System/TrackSystem/Track_Default_Master.Track_Default_Master_C")))
            (Variables|Default|SetIsBlocked true)
            (Rendering|Material|SetMaterial _preview_mesh 0 "/Game/Trap_System/Building_System/M_BuildingPreviewNotPlaceAbale.M_BuildingPreviewNotPlaceAbale")
            (Rendering|Material|SetMaterial _preview_mesh 1 "/Game/Trap_System/Building_System/M_BuildingPreviewNotPlaceAbale.M_BuildingPreviewNotPlaceAbale")
            (else
              (Variables|Default|SetIsBlocked false)
              (Rendering|Material|SetMaterial _preview_mesh 0 "/Game/Trap_System/Building_System/M_BuildingPreview.M_BuildingPreview")
              (Rendering|Material|SetMaterial _preview_mesh 1 "/Game/Trap_System/Building_System/M_BuildingPreview.M_BuildingPreview"))))
        (:then_2
          (Transformation|SetWorldTransform _preview_mesh _output_get false false))))))

(event Custom|ResetBuildMode
  (Utilities|FlowControl|DoOnce false) ; enters at Reset
)

(event Custom|Begin%20Build
  (bind _asplayer_controller (Utilities|Casting|CastToPlayerController (Pawn|GetController (stale EventBeginPlay _asbp_topdown))))
  (Input|RemoveMappingContext (PlayerController|LocalPlayerSubsystems|GetEnhancedInputLocalPlayerSubsystem _asplayer_controller) "/Game/Car/Inputs/IMC_Kart.IMC_Kart" "(bIgnoreAllPressedKeysUntilRelease=True,bForceImmediately=False,bNotifyUserSettings=False)")
  (Input|AddMappingContext (PlayerController|LocalPlayerSubsystems|GetEnhancedInputLocalPlayerSubsystem _asplayer_controller) "/Game/Trap_System/TopDownView/Inputs/IM_Movement.IM_Movement" 0 "(bIgnoreAllPressedKeysUntilRelease=True,bForceImmediately=False,bNotifyUserSettings=False)")
  (bind _returnvalue (UserInterface|CreateWidget "/Game/Trap_System/TopDownView/WB_TrapSelection.WB_TrapSelection_C" _asplayer_controller))
  (Default|SetPlayer _returnvalue (Variables|Default|GetPlayer))
  (bind _output_get (Variables|Default|SetTrapBuildingWIdget _returnvalue))
  (UserInterface|Viewport|AddtoPlayerScreen _output_get)
  (CallFunction|ServerCreateStaticMesh :topdown (Variables|Default|GetPlayer) :mesh (Variables|Default|GetStaticMeshBuild)))

(event Custom|StopBuildMode
  (Variables|Default|SetInBuildMode false)
  (bind _preview_mesh (Variables|Default|GetPreview%20Mesh)
    (:then
      (Components|StaticMesh|SetStaticMesh _preview_mesh 0)
      (Variables|Default|SetPreview%20Mesh 0)
      (CallFunction|ResetBuildMode))
    (:else)))

(event Custom|Rotate%20Preview)

(event Custom|RPC_SpawnActor
  (params (transform :type Transform) (trap :type BP%20Trap%20Master%20Class%20Reference))
  (Game|SpawnActorfromClass trap transform "AlwaysSpawn" "OverrideRootScale" 0 0)
  (Variables|Default|SetInBuildMode false)
  (Components|StaticMesh|SetStaticMesh (Variables|Default|GetPreview%20Mesh) 0)
  (bind _asstate_race (Utilities|Casting|CastToState_Race (Game|GetGameState)))
  (Default|AddPlayertoFinishedBuilding _asstate_race (Variables|Default|GetPlayer)))

(event Custom|RPC_Server_SpawnActor
  (params (transform :type Transform) (trap :type BP%20Trap%20Master%20Class%20Reference))
  (CallFunction|RPCSpawnActor transform trap))

(event Custom|PreviewBuild
  (params (transform :type Transform) (mesh :type Static%20Mesh%20Component%20Object%20Reference) (hit :type Boolean)))

(event Custom|ServerPreviewBuild
  (params (transform :type Transform) (mesh :type Static%20Mesh%20Component%20Object%20Reference) (hit :type Boolean))
  (CallFunction|PreviewBuild transform mesh hit))

(event Custom|ServerCreateStaticMesh
  (params (topdown :type BP%20Topdown%20Object%20Reference) (Transform :type Transform) (mesh :type Static%20Mesh%20Object%20Reference))
  (CallFunction|CreateStaticMesh topdown Transform mesh))

(event Custom|CreateStaticMesh
  (params (topdown :type BP%20Topdown%20Object%20Reference) (Transform :type Transform) (mesh :type Static%20Mesh%20Object%20Reference))
  (bind _returnvalue (Game|AddComponentbyClass topdown "/Script/Engine.StaticMeshComponent" false Transform))
  (Rendering|Material|SetMaterial _returnvalue 0 "/Game/Trap_System/Building_System/M_BuildingPreview.M_BuildingPreview")
  (Rendering|Material|SetMaterial _returnvalue 1 "/Game/Trap_System/Building_System/M_BuildingPreview.M_BuildingPreview")
  (Components|StaticMesh|SetStaticMesh _returnvalue mesh)
  (Collision|SetCollisionEnabled _returnvalue "NoCollision")
  (Variables|Default|SetPreview%20Mesh _returnvalue)
  (Variables|Default|SetBoxTraceHalfSize (.BoxExtent (Collision|GetComponentBounds _returnvalue)))
  (CallFunction|PreviewLoop))

(event Input|EnhancedActionEvents|EnhancedInputActionIA_PlaceBuild
  (params (ActionValue :type Boolean) (ElapsedSeconds :type Float%20%28double-precision%29) (TriggeredSeconds :type Float%20%28double-precision%29) (InputAction :type Input%20Action%20Object%20Reference :default "/Game/Trap_System/TopDownView/Inputs/IA_PlaceBuild.IA_PlaceBuild"))
  (:Started
    (if (Variables|Default|GetInBuildMode)
      (if (not (Variables|Default|GetIsBlocked))
        (CallFunction|RPCServerSpawnActor (Variables|Default|GetBuild%20Preview%20Transform) (Variables|Default|GetTrapClassBuild)))
      (elif (Variables|Default|GetinSelectMode)
        (bind _asstate_race (Utilities|Casting|CastToState_Race (Game|GetGameState)))
        (Variables|Default|SetInBuildSelect false)
        (Default|RemoveTrapfromAllPlayers _asstate_race (Variables|/Game/Trap_System/TopDownView/WB_TrapSelection.WB_TrapSelection_C|GetIndex (Variables|Default|GetTrapBuildingWIdget)))
        (Default|AddPlayertoFinishedBuildingSelection _asstate_race (Variables|Default|GetPlayer))
        (Widget|RemovefromParent (Variables|Default|GetTrapBuildingWIdget))))))

(event Input|EnhancedActionEvents|EnhancedInputActionIA_rotate
  (params (ActionValue :type Boolean) (ElapsedSeconds :type Float%20%28double-precision%29) (TriggeredSeconds :type Float%20%28double-precision%29) (InputAction :type Input%20Action%20Object%20Reference :default "/Game/Trap_System/TopDownView/Inputs/IA_rotate.IA_rotate"))
  (if (Variables|Default|GetInBuildMode)
    (Variables|Default|SetBuild%20Preview%20Rotation (Math|Rotator|CombineRotators (.rotation (Variables|Default|GetBuild%20Preview%20Transform)) "0.000000,90.000000,0.000000"))))

(event Input|EnhancedActionEvents|EnhancedInputActionIA_rotate2
  (params (ActionValue :type Vector%202D%20Structure) (ElapsedSeconds :type Float%20%28double-precision%29) (TriggeredSeconds :type Float%20%28double-precision%29) (InputAction :type Input%20Action%20Object%20Reference :default "/Game/Trap_System/TopDownView/Inputs/IA_rotate2.IA_rotate2"))
  (bind _controllersensitivity (Variables|Default|GetControllerSensitivity))
  (bind _asplayer_controller (Utilities|Casting|CastToPlayerController (Pawn|GetController (Variables|Default|GetPlayer))))
  (Class|PlayerController|SetMouseLocation (Game|GetPlayerController 0) (Math|Float|Round (+ (.LocationX (Game|Player|GetMousePosition _asplayer_controller)) (* (.y ActionValue) _controllersensitivity))) (Math|Float|Round (+ (.LocationY (Game|Player|GetMousePosition _asplayer_controller)) (* (.x ActionValue) (* _controllersensitivity -1.0))))))

(event Input|EnhancedActionEvents|EnhancedInputActionIA_ControllerMouse
  (params (ActionValue :type Boolean) (ElapsedSeconds :type Float%20%28double-precision%29) (TriggeredSeconds :type Float%20%28double-precision%29) (InputAction :type Input%20Action%20Object%20Reference :default "/Game/Trap_System/TopDownView/Inputs/IA_ControllerMouse.IA_ControllerMouse")))

(event Input|EnhancedActionEvents|EnhancedInputActionIA_Build
  (params (ActionValue :type Boolean) (ElapsedSeconds :type Float%20%28double-precision%29) (TriggeredSeconds :type Float%20%28double-precision%29) (InputAction :type Input%20Action%20Object%20Reference :default "/Game/Trap_System/TopDownView/Inputs/IA_Build.IA_Build")))

(event Input|EnhancedActionEvents|EnhancedInputActionIA_NextTrap
  (params (ActionValue :type Float%20%28double-precision%29) (ElapsedSeconds :type Float%20%28double-precision%29) (TriggeredSeconds :type Float%20%28double-precision%29) (InputAction :type Input%20Action%20Object%20Reference :default "/Game/Trap_System/TopDownView/Inputs/IA_NextTrap.IA_NextTrap"))
  (bind _trapbuildingwidget (Variables|Default|GetTrapBuildingWIdget))
  (if (Variables|Default|GetinSelectMode)
    (if (> ActionValue 0.0)
      (Default|NextTrap _trapbuildingwidget)
      (else
        (Default|PreviousTrap _trapbuildingwidget)))
    (CallFunction|PreviewLoop)))

(event EventBeginPlay
  (bind _asbp_topdown (Utilities|Casting|CastToBP_Topdown (Components|GetOwner)))
  (Variables|Default|SetPlayer _asbp_topdown)
  (Variables|Default|SetCamera (Variables|/Game/Trap_System/TopDownView/BP_Topdown.BP_Topdown_C|GetCamera _asbp_topdown)))

(event EventTick
  (params (DeltaSeconds :type Float%20%28single-precision%29))
  (if (Variables|Default|GetInBuildMode)
    (CallFunction|PreviewLoop)))

(fn GetGridLocation
  (params (Location :type Vector))
  (bind _grid_size (Variables|Default|GetGrid_Size))
  (bind _grid_size_2 (Variables|Default|GetGrid_Size))
  (bind _grid_size_3 (Variables|Default|GetGrid_Size))
  (bind _grid_offset (Variables|Default|GetGrid_Offset))
  (bind _returnvalue (/ _grid_size_2 2.0))
  (bind _returnvalue_2 (/ _grid_size_3 2.0))
  (return (Math|Vector|MakeVector (+ (* (Math|Conversions|ToFloat(Integer) (Math|Float|Round (/ (- (- (.x Location) _returnvalue) (.x _grid_offset)) _grid_size))) _grid_size_3) _returnvalue_2) (+ (* (Math|Conversions|ToFloat(Integer) (Math|Float|Round (/ (- (- (.y Location) _returnvalue) (.y _grid_offset)) _grid_size))) _grid_size_3) _returnvalue_2) (.z Location))))

(fn GetLocationUnderCursor
  (bind _returnvalue (Class|GameplayStatics|GetPlayerControllerfromID))
  (bind _hitresult (Game|Player|GetHitResultUnderCursorbyChannel _returnvalue "TraceTypeQuery1" true))
  (bind (_bblockinghit _binitialoverlap _time _distance _location) (Collision|BreakHitResult _hitresult))
  (bind (_x _y _z) (Math|Vector|BreakVector _location))
  (bind (_x_2 _y_2) (Math|Vector|BreakVector _location))
  (Class|WidgetLayoutLibrary|GetMousePositiononViewport)
  (bind _outhit (Collision|LineTraceByChannel (Math|Vector|MakeVector _x _y (.z (Transformation|GetWorldLocation (Variables|/Game/Trap_System/TopDownView/BP_Topdown.BP_Topdown_C|GetCamera (Variables|Default|GetPlayer))))) (Math|Vector|MakeVector _x _y (- _z 2e+01)) "TraceTypeQuery1" false 0 "None"))
  (if (Utilities|ClassIsChildOf (Utilities|GetClass (.HitActor (Collision|BreakHitResult _outhit))) "/Game/Trap_System/Traps/BP_TrapMaster.BP_TrapMaster_C")
    (return _bblockinghit (Math|Vector|MakeVector _x_2 _y_2 (.z (Transformation|GetActorLocation (.HitActor (Collision|BreakHitResult _outhit))))))
    (else
      (return false _location))))

(fn ChangeStaticMesh
  (params (Static%20Mesh :type Static%20Mesh%20Object%20Reference) (Comp :type Static%20Mesh%20Component%20Object%20Reference))
  (bind _preview_mesh (Variables|Default|GetPreview%20Mesh))
  (bind _output_get (Variables|Default|SetStaticMeshBuild Static%20Mesh))
  (Components|StaticMesh|SetStaticMesh _preview_mesh _output_get)
  (Variables|Default|SetBoxTraceHalfSize (.BoxExtent (Collision|GetComponentBounds _preview_mesh))))

(fn SetTrapClass
  (params (Trap%20Class :type BP%20Trap%20Master%20Class%20Reference))
  (Variables|Default|SetTrapClassBuild Trap%20Class))

(fn SetKartMaster
  (params (KartMaster :type BP%20Kart%20Object%20Reference))
  (Variables|Default|SetKartMaster KartMaster))

(fn ChangetoKart
  (bind _kartmaster (Variables|Default|GetKartMaster))
  (bind _asplayer_controller (Utilities|Casting|CastToPlayerController (Pawn|GetController (Variables|Default|GetPlayer))))
  (Pawn|Possess _asplayer_controller _kartmaster)
  (Default|RedoControlls _kartmaster)
  (Actor|DestroyActor (Variables|Default|GetPlayer))
  (return))