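; BP_Trap_Fan is a fan trap that pushes characters caught in its box along the direction of its arrow.
; Every Tick it polls the Box for overlapping actors and casts them to Temp_Char.
; It applies a constant force along the Arrow's forward vector to the character's capsule, as an acceleration change that ignores mass.
; The box's begin-overlap event is empty, so all logic runs on Tick.
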(event OnComponentBeginOverlap(Box)
  (params (OverlappedComponent :type Primitive%20Component%20Object%20Reference) (OtherActor :type Actor%20Object%20Reference) (OtherComp :type Primitive%20Component%20Object%20Reference) (OtherBodyIndex :type Integer) (bFromSweep :type Boolean) (SweepResult :type Hit%20Result%20Structure%20%28by%20ref%29)))

(event EventBeginPlay
  (|CallParentFunction) ; This node is disabled and will not be called.\nDrag off pins to build functionality.
)

(event Collision|EventActorBeginOverlap
  (params (OtherActor :type Actor%20Object%20Reference))
  (|CallParentFunction OtherActor) ; This node is disabled and will not be called.\nDrag off pins to build functionality.
)

(event EventTick
  (params (DeltaSeconds :type Float%20%28single-precision%29))
  (|CallParentFunction DeltaSeconds)
  (for _array_element (Collision|GetOverlappingActors (Variables|Default|GetBox) 0 :!class /Script/Engine.PrimitiveComponent)
    (bind _astemp_char (Utilities|Casting|CastToTemp_Char _array_element))
    (Physics|AddForce (Variables|/Script/Engine.Character|GetCapsuleComponent _astemp_char) (* (Math|Vector|GetForwardVector (Transformation|GetWorldRotation (Variables|Default|GetArrow))) 1e+03) "None" true)))

(fn ConstructionScript
  (|CallParentFunction))